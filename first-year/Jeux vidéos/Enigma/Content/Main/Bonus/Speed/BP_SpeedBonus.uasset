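; Speed bonus pickup that boosts a player who touches it.
; When a BP_Player overlaps its sphere while the pickup is available, it calls IncreaseSpeed on that player.
; It then hides its Niagara effect and blocks further pickups, re-enabling both after a five-second delay so it respawns in place.
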(event OnComponentBeginOverlap(Sphere)
  (params (OverlappedComponent :type Primitive%20Component%20Object%20Reference) (OtherActor :type Actor%20Object%20Reference) (OtherComp :type Primitive%20Component%20Object%20Reference) (OtherBodyIndex :type Integer) (bFromSweep :type Boolean) (SweepResult :type Hit%20Result%20Structure%20%28by%20ref%29))
  (bind _asbp_player (Utilities|Casting|CastToBP_Player OtherActor))
  (if (Variables|Default|GetCanBeTaken?)
    (Default|IncreaseSpeed _asbp_player)
    (Variables|Default|SetCanBeTaken? false)
    (Rendering|SetVisibility (Variables|Default|GetNS_Pickup_2) false false)
    (Utilities|FlowControl|Delay 5.0)
    (Variables|Default|SetCanBeTaken? true)
    (Rendering|SetVisibility (Variables|Default|GetNS_Pickup_2) true false)))

(event EventBeginPlay)

(event Collision|EventActorBeginOverlap
  (params (OtherActor :type Actor%20Object%20Reference)))

(event EventTick
  (params (DeltaSeconds :type Float%20%28single-precision%29)))

(fn ConstructionScript)