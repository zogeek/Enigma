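; Falling platform that shakes when the player character steps into its trigger box, then drops and respawns.
; Overlap plays a timeline that rolls the cube, with a DoOnce limiting the shake sound to once per cycle.
; When the timeline ends the cube simulates physics, then after a delay teleports to its transform saved at BeginPlay and re-arms the trigger and sound.
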(event OnComponentBeginOverlap(Box)
  (params (OverlappedComponent :type Primitive%20Component%20Object%20Reference) (OtherActor :type Actor%20Object%20Reference) (OtherComp :type Primitive%20Component%20Object%20Reference) (OtherBodyIndex :type Integer) (bFromSweep :type Boolean) (SweepResult :type Hit%20Result%20Structure%20%28by%20ref%29))
  (if (and (== OtherActor (Game|GetPlayerCharacter 0)) (Variables|Default|GetCanBeActivated?))
    (Variables|Default|SetCanBeActivated? false)
    (bind _shakerotation (Timeline|ShakePlatform PlayFromStart)
      (:Update
        (Transformation|SetWorldRotation (Variables|Default|GetCube) (Math|Rotator|MakeRotator _shakerotation 0.0 0.0) false false)
        (if (>= _shakerotation 0.8)
          (Utilities|FlowControl|DoOnce false
            (:Completed
              (Audio|PlaySound2D "/Game/StarterContent/Audio/Explosion01.Explosion01" 1.0 1.0 0.0 0 0)))))
      (:Finished
        (Physics|SetSimulatePhysics (Variables|Default|GetCube) true)
        (Utilities|FlowControl|Delay 5.0)
        (Physics|SetSimulatePhysics (Variables|Default|GetCube) false)
        (Transformation|SetWorldTransform (Variables|Default|GetCube) (Variables|Default|GetDefaultRespawnTransform) false true)
        (Variables|Default|SetCanBeActivated? true)
        (CallFunction|ResetDoOnceSFXShakePlatform)))))

(event Custom|ResetDoOnceSFXShakePlatform
  (Utilities|FlowControl|DoOnce false) ; enters at Reset
)

(event EventBeginPlay
  (Variables|Default|SetDefaultRespawnTransform (Transformation|GetWorldTransform (Variables|Default|GetCube))))

(fn ConstructionScript)