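; BP_AI is an AI pawn that patrols through the points in its PatrolRoute array.
; Tick issues AIMoveTo toward the current point, and on success a short Delay precedes advancing IndexRoute and looping back into the move.
; The index resets once it reaches the array length, checked before incrementing, so it steps one past the last point before wrapping.
; A failed move has no handler of its own.
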(event EventTick
  (params (DeltaSeconds :type Float%20%28single-precision%29))
  (AI|AIMoveTo self (Utilities|Array|Get(acopy) (Variables|Default|GetPatrolRoute) (Variables|Default|GetIndexRoute)) 0 5.0 false :!label _label
    (:OnSuccess
      (Utilities|FlowControl|Delay 2.0)
      (if (>= (Variables|Default|GetIndexRoute) (Utilities|Array|Length (Variables|Default|GetPatrolRoute)))
        (Variables|Default|SetIndexRoute 0)
        (goto _label)
        (else
          (Math|Integer|IncrementInt (Variables|Default|GetIndexRoute)
            (:%20%20
              (goto _label))))))))

(fn ConstructionScript)