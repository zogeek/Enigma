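; Master trigger zone actor whose zone type decides what happens when BP_Player enters its box.
; Dead zones respawn the player, checkpoints save the Arrow component's world transform as the player's last spawn, and win zones signal that the player has finished.
; Independently of zone type, any BP_SphereToSpawn that stops overlapping the box is destroyed.
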(event OnComponentBeginOverlap(Box)
  (params (OverlappedComponent :type Primitive%20Component%20Object%20Reference) (OtherActor :type Actor%20Object%20Reference) (OtherComp :type Primitive%20Component%20Object%20Reference) (OtherBodyIndex :type Integer) (bFromSweep :type Boolean) (SweepResult :type Hit%20Result%20Structure%20%28by%20ref%29))
  (bind _asbp_player (Utilities|Casting|CastToBP_Player OtherActor))
  (switch Utilities|FlowControl|Switch|SwitchonE_TriggerZone (Variables|Default|GetTriggerZone)
    (:NewEnumerator0
      (Default|Respawn _asbp_player))
    (:NewEnumerator1
      (Default|SetNewLastSpawnTransform _asbp_player (Transformation|GetWorldTransform (Variables|Default|GetArrow))))
    (:NewEnumerator2
      (Default|CallPlayerHasFinished))))

(event OnComponentEndOverlap(Box)
  (params (OverlappedComponent :type Primitive%20Component%20Object%20Reference) (OtherActor :type Actor%20Object%20Reference) (OtherComp :type Primitive%20Component%20Object%20Reference) (OtherBodyIndex :type Integer))
  (bind _asbp_sphere_to_spawn (Utilities|Casting|CastToBP_SphereToSpawn OtherActor))
  (Actor|DestroyActor _asbp_sphere_to_spawn))

(event EventBeginPlay)

(event Collision|EventActorBeginOverlap
  (params (OtherActor :type Actor%20Object%20Reference)))

(event EventTick
  (params (DeltaSeconds :type Float%20%28single-precision%29)))

(fn ConstructionScript)