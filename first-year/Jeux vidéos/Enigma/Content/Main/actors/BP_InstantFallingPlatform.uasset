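; BP_InstantFallingPlatform is a platform that drops with no delay when the player touches its trigger.
; A Box overlap from player character 0 clears CanBeActivated, so it fires only once, and turns on physics simulation for the Cube.
; BeginPlay stores the Cube's world transform as DefaultRespawnTransform, but nothing in these graphs restores it or re-arms the trigger.
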(event OnComponentBeginOverlap(Box)
  (params (OverlappedComponent :type Primitive%20Component%20Object%20Reference) (OtherActor :type Actor%20Object%20Reference) (OtherComp :type Primitive%20Component%20Object%20Reference) (OtherBodyIndex :type Integer) (bFromSweep :type Boolean) (SweepResult :type Hit%20Result%20Structure%20%28by%20ref%29))
  (if (and (== OtherActor (Game|GetPlayerCharacter 0)) (Variables|Default|GetCanBeActivated?))
    (Variables|Default|SetCanBeActivated? false)
    (Physics|SetSimulatePhysics (Variables|Default|GetCube) true)))

(event EventBeginPlay
  (Variables|Default|SetDefaultRespawnTransform (Transformation|GetWorldTransform (Variables|Default|GetCube))))

(fn ConstructionScript)