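; BP_Turn is a rotating bumper obstacle that launches the player on contact.
; On BeginPlay, a timeline with configurable speed and start offset drives the cylinder's yaw around a fixed 90-degree pitch, with an Inversed flag reversing the direction.
; When BP_Player overlaps the capsule, its movement component receives a fixed diagonal velocity-change impulse, independent of the bumper's rotation or the hit direction.
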(event OnComponentBeginOverlap(Capsule)
  (params (OverlappedComponent :type Primitive%20Component%20Object%20Reference) (OtherActor :type Actor%20Object%20Reference) (OtherComp :type Primitive%20Component%20Object%20Reference) (OtherBodyIndex :type Integer) (bFromSweep :type Boolean) (SweepResult :type Hit%20Result%20Structure%20%28by%20ref%29))
  (bind _asbp_player (Utilities|Casting|CastToBP_Player OtherActor))
  (Physics|AddImpulse (Variables|/Script/Engine.Character|GetCharacterMovement _asbp_player) "500.000000,500.000000,500.000000" true))

(event EventBeginPlay
  (bind _cylinder1 (Variables|Default|GetCylinder1))
  (Components|Timeline|SetPlayRate (Variables|Default|GetBumper_Rotation) (Variables|Default|GetSpeed))
  (Components|Timeline|SetNewTime (Variables|Default|GetBumper_Rotation) (Variables|Default|GetStartOffSet))
  (bind _rotation (Timeline|Bumper_Rotation Play)
    (:Update
      (if (Variables|Default|GetInversed)
        (Transformation|SetRelativeRotation _cylinder1 (Math|Rotator|MakeRotator 0.0 9e+01 (* _rotation -1.0)) false false)
        (else
          (Transformation|SetRelativeRotation _cylinder1 (Math|Rotator|MakeRotator 0.0 9e+01 _rotation) false false))))))

(fn ConstructionScript)